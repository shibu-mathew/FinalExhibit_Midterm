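; Red Light, Green Light hazard that sends the player back to a checkpoint for moving during red light.
; A looping timeline drives the RectLight color and sets the red-light flag while the red channel is exactly 1.
; Overlaps on the motion detector collider set an inside flag, and Tick checks the overlapping character's velocity against a small threshold during red.
; An older delay-based, randomized light sequence remains unconnected.
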(event OnComponentBeginOverlap(Collider_MotionDetector)
  (params (OverlappedComponent :type Primitive%20Component%20Object%20Reference) (OtherActor :type Actor%20Object%20Reference) (OtherComp :type Primitive%20Component%20Object%20Reference) (OtherBodyIndex :type Integer) (bFromSweep :type Boolean) (SweepResult :type Hit%20Result%20Structure%20%28by%20ref%29))
  (Variables|Default|SetIsInside true))

(event OnComponentEndOverlap(Collider_MotionDetector)
  (params (OverlappedComponent :type Primitive%20Component%20Object%20Reference) (OtherActor :type Actor%20Object%20Reference) (OtherComp :type Primitive%20Component%20Object%20Reference) (OtherBodyIndex :type Integer))
  (Variables|Default|SetIsInside false))

(event EventBeginPlay
  (bind _color (Timeline|Timeline Play)
    (:Update
      (Rendering|Components|Light|SetLightColor (Variables|Default|GetRectLight) (Utilities|Struct|MakeLinearColor (.x _color) (.y _color) (.z _color) 1.0) true)
      (if (== (.x _color) 1.0)
        (Variables|Default|SetIsRedLight true)
        (else
          (Variables|Default|SetIsRedLight false))))
    (:Finished
      (Utilities|FlowControl|Delay 0.2)
      (Timeline|Timeline PlayFromStart))))

(event EventTick
  (params (DeltaSeconds :type Float%20%28single-precision%29))
  (if (Variables|Default|GetIsInside)
    (if (Variables|Default|GetIsRedLight)
      (bind _asbp_third_person_character (Utilities|Casting|CastToBP_ThirdPersonCharacter (stale OnComponentBeginOverlap(Collider_MotionDetector) OtherActor)))
      (if (< 5.0 (Math|Vector|VectorLength (Variables|/Script/Engine.MovementComponent|GetVelocity (Variables|/Script/Engine.Character|GetCharacterMovement _asbp_third_person_character))))
        (Default|RespawnCheckpoint (Variables|Default|GetCheckpointSystem) _asbp_third_person_character)))))

(fn ConstructionScript)