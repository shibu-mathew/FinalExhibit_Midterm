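; BP_Gate is a gate actor that slides its SMGate mesh vertically to open and close.
; OpenGate and CloseGate events each play a sound at the actor's location and run their own timeline.
; Each timeline's track drives a Lerp that sets the mesh's relative Z between the closed and raised positions.
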(event Custom|OpenGate
  (Audio|PlaySoundatLocation "/Engine/VREditor/Sounds/UI/Enter_Simulate.Enter_Simulate" (Transformation|GetActorLocation) "0, 0, 0" 1.0 1.0 0.0 0 0 0 0)
  (bind _track_open (Timeline|Timeline_Open Play)
    (:Update
      (Transformation|SetRelativeLocation (Variables|Default|GetSM_Gate) (Math|Vector|MakeVector 0.0 0.0 (Math|Float|Lerp 0.0 2e+02 _track_open)) false false))))

(event Custom|CloseGate
  (Audio|PlaySoundatLocation "/Engine/VREditor/Sounds/UI/Leave_Simulate.Leave_Simulate" (Transformation|GetActorLocation) "0, 0, 0" 1.0 1.0 0.0 0 0 0 0)
  (bind _track_close (Timeline|Timeline_Close Play)
    (:Update
      (Transformation|SetRelativeLocation (Variables|Default|GetSM_Gate) (Math|Vector|MakeVector 0.0 0.0 (Math|Float|Lerp 0.0 2e+02 _track_close)) false false))))

(fn ConstructionScript)