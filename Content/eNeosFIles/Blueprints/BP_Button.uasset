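; BP_Button is a one-shot interactable button that opens a linked gate, and optionally a fence, for the third-person character.
; On Interact, it sets the character's ButtonDisabled flag, then a DoOnce plays a sound and swaps the button mesh to its enabled material.
; After a short delay it opens TargetGate and marks itself Disabled, then after another delay opens TargetFence if that reference is valid.
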(event EventInteract
  (params (OtherActor :type Actor%20Object%20Reference))
  (bind _targetfence (Variables|Default|GetTargetFence))
  (bind _asbp_third_person_character (Utilities|Casting|CastToBP_ThirdPersonCharacter OtherActor))
  (Variables|/Game/ThirdPerson/Blueprints/BP_ThirdPersonCharacter.BP_ThirdPersonCharacter_C|SetButtonDisabled _asbp_third_person_character true)
  (Utilities|FlowControl|DoOnce false
    (:Completed
      (Audio|PlaySoundatLocation "/Engine/EditorSounds/Notifications/CompileSuccess.CompileSuccess" (Transformation|GetActorLocation) "0, 0, 0" 1.0 1.0 0.0 0 0 0 0)
      (Rendering|Material|SetMaterial (Variables|Default|GetSM_Button) 0 "/Game/eNeosFIles/Materials/MAT_ButtonEnabled.MAT_ButtonEnabled")
      (Utilities|FlowControl|Delay 1.0)
      (Default|OpenGate (Variables|Default|GetTargetGate))
      (Variables|Default|SetDisabled true)
      (Utilities|FlowControl|Delay 1.0)
      (Utilities|IsValid _targetfence
        (:Is%20Valid
          (Default|OpenFence _targetfence))))))

(fn ConstructionScript)