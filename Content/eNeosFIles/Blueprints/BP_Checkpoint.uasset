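; BP_Checkpoint is a two-sided checkpoint actor that respawns an actor on one of two sides, depending on whether the hub has been exited.
; When BP_ThirdPersonCharacter overlaps collider A or B, it sets BoolExitedHub true or false and stores that collider's world location plus an offset.
; The RespawnCheckpoint event uses that flag to move the supplied actor to RespawnA or RespawnB.
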(event OnComponentBeginOverlap(Collider_CheckpointB)
  (params (OverlappedComponent :type Primitive%20Component%20Object%20Reference) (OtherActor :type Actor%20Object%20Reference) (OtherComp :type Primitive%20Component%20Object%20Reference) (OtherBodyIndex :type Integer) (bFromSweep :type Boolean) (SweepResult :type Hit%20Result%20Structure%20%28by%20ref%29))
  (bind _offsetb (Variables|Default|GetOffsetB))
  (bind _collider_checkpointb (Variables|Default|GetCollider_CheckpointB))
  (bind _returnvalue (Transformation|GetWorldLocation _collider_checkpointb))
  (Utilities|Casting|CastToBP_ThirdPersonCharacter OtherActor)
  (Variables|Default|Setbool_ExitedHub false)
  (Variables|Default|SetRespawnB (Math|Vector|MakeVector (+ (.x _offsetb) (.x _returnvalue)) (+ (.y _offsetb) (.y _returnvalue)) (+ (.z _offsetb) (.z _returnvalue)))))

(event OnComponentBeginOverlap(Collider_CheckpointA)
  (params (OverlappedComponent :type Primitive%20Component%20Object%20Reference) (OtherActor :type Actor%20Object%20Reference) (OtherComp :type Primitive%20Component%20Object%20Reference) (OtherBodyIndex :type Integer) (bFromSweep :type Boolean) (SweepResult :type Hit%20Result%20Structure%20%28by%20ref%29))
  (bind _collider_checkpointa (Variables|Default|GetCollider_CheckpointA))
  (bind _offseta (Variables|Default|GetOffsetA))
  (bind _returnvalue (Transformation|GetWorldLocation _collider_checkpointa))
  (Utilities|Casting|CastToBP_ThirdPersonCharacter OtherActor)
  (Variables|Default|Setbool_ExitedHub true)
  (Variables|Default|SetRespawnA (Math|Vector|MakeVector (+ (.x _offseta) (.x _returnvalue)) (+ (.y _offseta) (.y _returnvalue)) (+ (.z _offseta) (.z _returnvalue)))))

(event Custom|RespawnCheckpoint
  (params (OtherActor :type Actor%20Object%20Reference))
  (if (Variables|Default|Getbool_ExitedHub)
    (Transformation|SetActorLocationAndRotation OtherActor (Variables|Default|GetRespawnA))
    (else
      (Transformation|SetActorLocationAndRotation OtherActor (Variables|Default|GetRespawnB)))))

(fn ConstructionScript)