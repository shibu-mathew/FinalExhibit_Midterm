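; BP_MiddleFence is a fence actor that sinks out of the way when something overlaps its capsule.
; Any overlap plays the Enter_Simulate sound and runs a timeline that lerps the fence mesh's relative Z downward.
; A second sound and timeline branch, apparently meant for closing, is disconnected, so nothing in the graph raises the fence again.
; The asset sits in an Unused folder.
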(event OnComponentBeginOverlap(Capsule)
  (params (OverlappedComponent :type Primitive%20Component%20Object%20Reference) (OtherActor :type Actor%20Object%20Reference) (OtherComp :type Primitive%20Component%20Object%20Reference) (OtherBodyIndex :type Integer) (bFromSweep :type Boolean) (SweepResult :type Hit%20Result%20Structure%20%28by%20ref%29))
  (Audio|PlaySoundatLocation "/Engine/VREditor/Sounds/UI/Enter_Simulate.Enter_Simulate" (Transformation|GetActorLocation) "0, 0, 0" 1.0 1.0 0.0 0 0 0 0)
  (bind _track_open (Timeline|Timeline Play)
    (:Update
      (Transformation|SetRelativeLocation (Variables|Default|GetSM_MiddleFence) (Math|Vector|MakeVector 0.0 0.0 (Math|Float|Lerp 0.0 -1.8e+02 _track_open)) false false))))

(event EventBeginPlay)

(event Collision|EventActorBeginOverlap
  (params (OtherActor :type Actor%20Object%20Reference)))

(event EventTick
  (params (DeltaSeconds :type Float%20%28single-precision%29)))

(fn ConstructionScript)