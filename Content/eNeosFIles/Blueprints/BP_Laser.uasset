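; BP_Laser is a laser hazard that sweeps back and forth or along a path and sends the player back on contact.
; After a start delay, a looping Timeline interpolates the laser mesh's height and pitch, parking it at its starting pose when Disable reports disabled.
; Overlap with the third-person character waits briefly, plays a sound, then respawns through CheckpointSystem, falling back to ResetPosition if none is valid.
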(event OnComponentBeginOverlap(Collision_Laser)
  (params (OverlappedComponent :type Primitive%20Component%20Object%20Reference) (OtherActor :type Actor%20Object%20Reference) (OtherComp :type Primitive%20Component%20Object%20Reference) (OtherBodyIndex :type Integer) (bFromSweep :type Boolean) (SweepResult :type Hit%20Result%20Structure%20%28by%20ref%29))
  (bind _checkpointsystem (Variables|Default|GetCheckpointSystem))
  (bind _asbp_third_person_character (Utilities|Casting|CastToBP_ThirdPersonCharacter OtherActor))
  (Utilities|FlowControl|Delay 0.5)
  (Audio|PlaySoundatLocation "/Engine/VREditor/Sounds/UI/Invalid_Action.Invalid_Action" (Transformation|GetActorLocation) "0, 0, 0" 1.0 1.0 0.0 0 0 0 0)
  (if (Utilities|IsValid _checkpointsystem)
    (Default|RespawnCheckpoint _checkpointsystem _asbp_third_person_character)
    (else
      (Transformation|SetActorLocationAndRotation _asbp_third_person_character (Variables|Default|GetResetPosition)))))

(event EventBeginPlay
  (bind _sm_laser (Variables|Default|GetSM_Laser))
  (bind _sm_laser_2 (Variables|Default|GetSM_Laser))
  (bind _returnvalue (Transformation|GetWorldLocation _sm_laser_2))
  (bind _returnvalue_2 (Transformation|GetWorldLocation _sm_laser))
  (Utilities|FlowControl|Delay (Variables|Default|GetStartDelay))
  (bind _track_sweep (Timeline|Timeline Play)
    (:Update
      (Transformation|SetWorldLocationAndRotation _sm_laser_2 (Math|Vector|MakeVector (.x _returnvalue) (.y _returnvalue) (Math|Float|Lerp (Variables|Default|GetHeightA) (Variables|Default|GetHeightB) _track_sweep)) (Math|Rotator|MakeRotator 0.0 (Math|Float|Lerp (Variables|Default|GetAngleA) (Variables|Default|GetAngleB) _track_sweep) 0.0) false false))
    (:Finished
      (Utilities|FlowControl|Delay 0.0)
      (if (Variables|/Game/eNeosFIles/Blueprints/BP_Button.BP_Button_C|GetDisabled (Variables|Default|GetDisable))
        (Transformation|SetWorldLocationAndRotation _sm_laser (Math|Vector|MakeVector (.x _returnvalue_2) (.y _returnvalue_2) (Variables|Default|GetHeightA)) (Math|Rotator|MakeRotator 0.0 (Variables|Default|GetAngleA) 0.0) false false)
        (else
          (Timeline|Timeline PlayFromStart))))))

(fn ConstructionScript)